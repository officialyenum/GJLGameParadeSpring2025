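; Base actor for interactable items, with an empty Interact event, a static mesh, a collision sphere and an info widget.
; At BeginPlay it hides the widget and passes itself to WBPC_ItemInfo as the item reference, with ToggleWidget controlling visibility.
; Sphere overlaps increment or decrement the overlapped-item count through the other actor's PlayerMessage, with debug prints.
; A Rotate event spins the mesh in yaw through a timeline.
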(event `self.ReceiveBeginPlay`
  (`self.ToggleWidget` false)
  (bind _aswbpc_item_info (cast `/Game/Core/Blueprint/Widgets/Components/WBPC_ItemInfo` (`WidgetComponent.GetUserWidgetObject` (`self.InfoWidget`))))
  (set `/Game/Core/Blueprint/Widgets/Components/WBPC_ItemInfo.ItemReference` self _aswbpc_item_info))

(event `Rotate`
  (`Timeline|RotateTimeline`
    (:`Update`
      (`SceneComponent.K2_AddWorldRotation` (`self.StaticMesh`) (`KismetMathLibrary.MakeRotator` 0.0 0.0 1.0) false false))))

(event `self.Sphere Collision.OnComponentBeginOverlap`
  (params (OverlappedComponent :type "PrimitiveComponent Object Reference") (OtherActor :type "Actor Object Reference") (OtherComp :type "PrimitiveComponent Object Reference") (OtherBodyIndex :type Integer) (bFromSweep :type Boolean) (SweepResult :type "HitResult Structure (by ref)"))
  (bind _player (message `/Game/Core/Blueprint/Interfaces/BPI_MainPlayer.GetPlayer` OtherActor))
  (`/Engine/EditorBlueprintResources/StandardMacros.IsValid` _player
    (:`Is Valid`
      (`/Game/Core/Blueprint/Character/BP_Player.IncrementItemOverlapped` _player 1)
      (`KismetSystemLibrary.PrintString` "Overlapped"))))

(event `self.Sphere Collision.OnComponentEndOverlap`
  (params (OverlappedComponent :type "PrimitiveComponent Object Reference") (OtherActor :type "Actor Object Reference") (OtherComp :type "PrimitiveComponent Object Reference") (OtherBodyIndex :type Integer))
  (bind _player (message `/Game/Core/Blueprint/Interfaces/BPI_MainPlayer.GetPlayer` OtherActor))
  (`/Engine/EditorBlueprintResources/StandardMacros.IsValid` _player
    (:`Is Valid`
      (`/Game/Core/Blueprint/Character/BP_Player.IncrementItemOverlapped` _player -1)
      (`KismetSystemLibrary.PrintString` "End Overlapped")
      (`KismetSystemLibrary.PrintString` (`KismetStringLibrary.Conv_IntToString` (`/Game/Core/Blueprint/Character/BP_Player.OverlappedItemCount` _player))))))

(event `/Game/Core/Blueprint/Interfaces/BPI_Interactable.Interact`)

(fn `ToggleWidget`
  (params (`bShow?` :type Boolean))
  (bind _infowidget (`self.InfoWidget`))
  (if `bShow?`
    (`SceneComponent.SetVisibility` _infowidget `bShow?` false)
    (else
      (`SceneComponent.SetVisibility` _infowidget `bShow?` false))))

(fn `UserConstructionScript`)