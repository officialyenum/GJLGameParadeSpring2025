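; BP_Pillar is a multi-part structure actor whose FixHouse event animates its pieces into place in stages.
; Six chained timelines set relative locations of Cube4, two cube pairs, Middle, Left and Right, mostly along Z.
; Each stage starts the next from its Update through a one-second Delay, so stages can overlap.
; Left's Lerp runs from zero to zero, so it snaps to a fixed position rather than animating.
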(event `FixHouse`
  (bind (_direction _newtrack_0) (`Timeline|Timeline`)
    (:`Update`
      (`SceneComponent.K2_SetRelativeLocation` (`self.Cube4`) (`KismetMathLibrary.MakeVector` 0.0 0.0 (- _newtrack_0 50.0)) false false)
      (`KismetSystemLibrary.Delay` 1.0)
      (bind (_direction_2 _newtrack_0_2) (`Timeline|Timeline_0`)
        (:`Update`
          (`SceneComponent.K2_SetRelativeLocation` (`self.Cube2`) (`KismetMathLibrary.MakeVector` 0.0 0.0 (- _newtrack_0_2 50.0)) false false)
          (`SceneComponent.K2_SetRelativeLocation` (`self.Cube1`) (`KismetMathLibrary.MakeVector` 0.0 0.0 (- _newtrack_0_2 50.0)) false false)
          (`KismetSystemLibrary.Delay` 1.0)
          (bind (_direction_3 _newtrack_0_3) (`Timeline|Timeline_1`)
            (:`Update`
              (`SceneComponent.K2_SetRelativeLocation` (`self.Cube`) (`KismetMathLibrary.MakeVector` 0.0 0.0 (- _newtrack_0_3 50.0)) false false)
              (`SceneComponent.K2_SetRelativeLocation` (`self.Cube3`) (`KismetMathLibrary.MakeVector` 0.0 0.0 (- _newtrack_0_3 50.0)) false false)
              (`KismetSystemLibrary.Delay` 1.0)
              (bind (_direction_4 _newtrack_0_4) (`Timeline|Timeline_2`)
                (:`Update`
                  (`SceneComponent.K2_SetRelativeLocation` (`self.Middle`) (`KismetMathLibrary.MakeVector` 0.0 0.0 (+ _newtrack_0_4 300.0)) false false)
                  (`KismetSystemLibrary.Delay` 1.0)
                  (bind (_direction_5 _newtrack_0_5) (`Timeline|Timeline_3`)
                    (:`Update`
                      (`SceneComponent.K2_SetRelativeLocation` (`self.Left`) (`KismetMathLibrary.MakeVector` 0.0 (`KismetMathLibrary.Lerp` 0.0 0.0 _newtrack_0_5) 550.0) false false)
                      (`KismetSystemLibrary.Delay` 1.0)
                      (bind (_direction_6 _newtrack_0_6) (`Timeline|Timeline_4`)
                        (:`Update`
                          (`SceneComponent.K2_SetRelativeLocation` (`self.Right`) (`KismetMathLibrary.MakeVector` 350.0 0.0 (+ _newtrack_0_6 550.0)) false false))))))))))))))

(fn `UserConstructionScript`)