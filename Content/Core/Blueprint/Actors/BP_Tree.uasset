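; BP_Tree is an interactable tree actor that tips over when the Interact event fires.
; PushTree plays a 2D hit sound and runs a timeline that lerps the roll of component W to a right angle while setting ItemAction to "Disabled".
; ActionHasBeenPerformed blocks further pushes, but is only set once the timeline finishes.
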(event `PushTree`
  (`GameplayStatics.PlaySound2D` "/Game/Core/Assets/Audios/Environments/Hit_Generic_5-1.Hit_Generic_5-1" 1.0 1.0 0.0 null null)
  (bind (_direction _newtrack_0) (`Timeline|Timeline_0` :!via `PlayFromStart`)
    (:`Update`
      (`SceneComponent.K2_SetRelativeRotation` (`self.w`) (`KismetMathLibrary.MakeRotator` (`KismetMathLibrary.Lerp` 0.0 90.0 _newtrack_0)) false false)
      (set `self.ItemAction` "Disabled"))
    (:`Finished`
      (set `self.bActionHasBeen Performed` true))))

(event `/Game/Core/Blueprint/Interfaces/BPI_Interactable.Interact`
  (if (not (`self.bActionHasBeen Performed`))
    (`self.PushTree`)))

(fn `UserConstructionScript`)