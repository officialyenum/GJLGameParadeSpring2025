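; BP_Plant is an interactable actor that plays a one-time planting movement and then opens a gate.
; Interact calls Plant, where a DoOnce starts the Planting timeline to drive StaticMesh1's relative height.
; Half a second after that timeline begins updating, a second DoOnce plays a creak sound and starts the Opens timeline, which swings the Gate's yaw.
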(event `/Game/Core/Blueprint/Interfaces/BPI_Interactable.Interact`
  (`self.Plant`))

(event `Plant`
  (`/Engine/EditorBlueprintResources/StandardMacros.DoOnce` false
    (:`Completed`
      (bind (_direction _plantin) (`Timeline|Planting`)
        (:`Update`
          (`SceneComponent.K2_SetRelativeLocation` (`self.StaticMesh1`) (`KismetMathLibrary.MakeVector` 0.0 0.0 (+ _plantin 100.0)) false false)
          (`KismetSystemLibrary.Delay` 0.5)
          (`/Engine/EditorBlueprintResources/StandardMacros.DoOnce` false
            (:`Completed`
              (`GameplayStatics.PlaySound2D` "/Game/Core/Assets/Audios/Environments/Wood_and_Door_Creak_01.Wood_and_Door_Creak_01" 1.0 1.0 0.0 null null)
              (bind (_direction_2 _newtrack_0) (`Timeline|opens`)
                (:`Update`
                  (`SceneComponent.K2_SetRelativeRotation` (`self.Gate`) (`KismetMathLibrary.MakeRotator` 0.0 0.0 (* _newtrack_0 30.0)) false false))))))))))

(fn `UserConstructionScript`)