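; One-shot trigger area that switches the player between the Grand Son and Grand Dad characters and teleports them to the new character's last position.
; On box overlap, the player's type and a direction flag select the transfer, and the area destroys itself afterwards.
; Each transfer saves the current transform in the game instance, flips the player type on the same actor, then applies the other character's stored transform.
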(event `self.ReceiveBeginPlay`
  (bind _game_instance (message `/Game/Core/Blueprint/Interfaces/BPI_GameInstance.GetGameInstance` (`GameplayStatics.GetGameInstance`)))
  (bind _output_get (set `self.Game InstanceRef` _game_instance))
  (`KismetSystemLibrary.PrintString` (`KismetSystemLibrary.GetDisplayName` _output_get) true true (struct :`G` 0.66 :`B` 1.0 :`A` 1.0) 5.0))

(event `self.Box.OnComponentBeginOverlap`
  (params (OverlappedComponent :type "PrimitiveComponent Object Reference") (OtherActor :type "Actor Object Reference") (OtherComp :type "PrimitiveComponent Object Reference") (OtherBodyIndex :type Integer) (bFromSweep :type Boolean) (SweepResult :type "HitResult Structure (by ref)"))
  (bind _player (message `/Game/Core/Blueprint/Interfaces/BPI_MainPlayer.GetPlayer` OtherActor))
  (switch `/Game/Core/Blueprint/Data/Enums/E_PlayerType` (`/Game/Core/Blueprint/Character/BP_Player.PlayerType` _player)
    (:`NewEnumerator0`
      (if (`self.bTeleportToGrandDad?`)
        (`self.TeleportToGrandDad` _player)
        (`self.K2_DestroyActor`)))
    (:`NewEnumerator1`
      (if (not (`self.bTeleportToGrandDad?`))
        (`self.TeleportToGrandSon` _player)
        (`self.K2_DestroyActor`)))))

(fn `TeleportToGrandDad`
  (params (PlayerRef :type "/Game/Core/Blueprint/Character/BP_Player Object Reference"))
  (if (`|EnumEquality` (`/Game/Core/Blueprint/Character/BP_Player.PlayerType` PlayerRef) "NewEnumerator0")
    (`/Game/Core/Blueprint/Game/BP_GameInstance.UpdatePlayerLastPosition` (`self.Game InstanceRef`) "NewEnumerator0" (`self.GetTransform` PlayerRef))
    (set `/Game/Core/Blueprint/Character/BP_Player.PlayerType` "NewEnumerator1" (`local.PlayerRef`))
    (`self.K2_SetActorTransform` (`local.PlayerRef`) (`/Game/Core/Blueprint/Game/BP_GameInstance.GetGrandDadLastPosition` (`self.Game InstanceRef`)) false false)
    (`KismetSystemLibrary.PrintString` "Is Grand Dad")))

(fn `TeleportToGrandSon`
  (params (PlayerRef :type "/Game/Core/Blueprint/Character/BP_Player Object Reference"))
  (if (`|EnumEquality` (`/Game/Core/Blueprint/Character/BP_Player.PlayerType` PlayerRef) "NewEnumerator1")
    (`/Game/Core/Blueprint/Game/BP_GameInstance.UpdatePlayerLastPosition` (`self.Game InstanceRef`) "NewEnumerator1" (`self.GetTransform` PlayerRef))
    (set `/Game/Core/Blueprint/Character/BP_Player.PlayerType` "NewEnumerator0" (`local.PlayerRef`))
    (`self.K2_SetActorTransform` (`local.PlayerRef`) (`/Game/Core/Blueprint/Game/BP_GameInstance.GetGrandSonLastPosition` (`self.Game InstanceRef`)) false false)
    (`KismetSystemLibrary.PrintString` "Is Grand Son")))

(fn `UserConstructionScript`)