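; BP_KeysAudio is a one-shot trigger that plays a scripted keys audio sequence when BP_Player enters its box.
; Box overlap runs through a DoOnce, spawning two 2D voice or sound cues with timed delays between them.
; A final wood and door creak plays alongside a timeline that yaws the static mesh, apparently swinging a door open.
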(event `self.Box.OnComponentBeginOverlap`
  (params (OverlappedComponent :type "PrimitiveComponent Object Reference") (OtherActor :type "Actor Object Reference") (OtherComp :type "PrimitiveComponent Object Reference") (OtherBodyIndex :type Integer) (bFromSweep :type Boolean) (SweepResult :type "HitResult Structure (by ref)"))
  (cast `/Game/Core/Blueprint/Character/BP_Player` OtherActor)
  (`/Engine/EditorBlueprintResources/StandardMacros.DoOnce` false
    (:`Completed`
      (`GameplayStatics.SpawnSound2D` "/Game/Core/Assets/Audios/Grandad/Future/The_Keys_Grandad_Cue.The_Keys_Grandad_Cue" 1.0 1.0 0.0 null)
      (`KismetSystemLibrary.Delay` 34.0)
      (`GameplayStatics.SpawnSound2D` "/Game/Core/Assets/Audios/Grandson/TheKeys_GS_Cue.TheKeys_GS_Cue" 1.0 1.0 0.0 null)
      (`KismetSystemLibrary.Delay` 10.0)
      (`GameplayStatics.PlaySound2D` "/Game/Core/Assets/Audios/Environments/Wood_and_Door_Creak_01.Wood_and_Door_Creak_01" 1.0 1.0 0.0 null null)
      (bind (_direction _newtrack_0) (`Timeline|Timeline`)
        (:`Update`
          (`SceneComponent.K2_SetRelativeRotation` (`self.StaticMesh`) (`KismetMathLibrary.MakeRotator` 0.0 0.0 (* _newtrack_0 40.0)) false false))))))

(fn `UserConstructionScript`)