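; Interactable actor that triggers the game's ending with end audio, a cinematic and the credits.
; On Interact, if ActionHasBeenPerformed is false, a DoOnce fires the grandad ending sound cue in 2D and plays the SequenceRoot level sequence.
; A fixed delay of just over a minute then adds the credits widget to the viewport, timed independently of the sound and sequence.
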(event `/Game/Core/Blueprint/Interfaces/BPI_Interactable.Interact`
  (if (not (`self.bActionHasBeen Performed`))
    (`/Engine/EditorBlueprintResources/StandardMacros.DoOnce` false
      (:`Completed`
        (`GameplayStatics.SpawnSound2D` "/Game/Core/Assets/Audios/Grandad/Future/The_End_Grandad_Cue.The_End_Grandad_Cue" 1.0 1.0 0.0 null)
        (`|ExecutionSequence`
          (:`then_0`
            (bind (_outactor _returnvalue) (`LevelSequencePlayer.CreateLevelSequencePlayer` "/Game/Cinematics/Sequences/Sequence/SequenceRoot.SequenceRoot"))
            (`MovieSceneSequencePlayer.Play` _returnvalue))
          (:`then_1`
            (`KismetSystemLibrary.Delay` 70.0)
            (bind _returnvalue_2 (`|CreateWidget` "/Game/Core/Blueprint/Widgets/Credits_WB.Credits_WB_C"))
            (`UserWidget.AddToViewport` _returnvalue_2 0)))))))

(fn `UserConstructionScript`)